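; BP_Samurai is a paper-sprite duelist in a reaction-timing duel, sliding into position at start and on reset.
; Attack checks the GM_Duel phase: pressing during Wait shows a cross and locks out further input, while Draw finishes the round.
; A winning draw timeline lunges the sprite forward, swaps it to the attack pose, and reports success and player control to the game mode.
; Defeated shows the defeated sprite.
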(event Custom|SlideIn
  (Components|Timeline|SetPlayRate (Variables|Default|GetSlideInAnim) 1.5)
  (bind _alpha (Timeline|SlideInAnim PlayFromStart)
    (:Update
      (Transformation|SetRelativeLocation (Variables|Default|GetPaperSprite) (Math|Vector|Lerp(Vector) (Variables|Default|GetSlideStartPos) (Variables|Default|GetSlideEndPos) _alpha) false false))))

(event Custom|Attack
  (if (not (Variables|Default|GetPressedDraw))
    (switch Utilities|FlowControl|Switch|SwitchonE_Phase (Variables|/Game/Blueprints/GM_Duel.GM_Duel_C|GetPhase (Variables|Default|GetAs%20GM%20Duel))
      (:NewEnumerator1
        (CallFunction|SetCrossVisibility true)
        (Variables|Default|SetPressedDraw true))
      (:NewEnumerator2
        (Variables|Default|SetPressedDraw true)
        (Default|SetGameFinish (Variables|Default|GetAs%20GM%20Duel))
        (Components|Timeline|SetPlayRate (Variables|Default|GetDrawCloser) 9.0)
        (bind _alpha (Timeline|DrawCloser Play)
          (:Update
            (Transformation|SetRelativeLocation (Variables|Default|GetPaperSprite) (Math|Vector|Lerp(Vector) (Variables|Default|GetSlideEndPos) (Variables|/Script/Engine.SceneComponent|GetRelativeLocation (Variables|Default|GetAttackPos)) _alpha) false false))
          (:SwitchSprite
            (Rendering|Components|Sprite|SetSprite (Variables|Default|GetPaperSprite) (Variables|Default|GetAttackedSprite))
            (Default|AttackSuccesfully (Variables|Default|GetAs%20GM%20Duel) (Pawn|IsPlayerControlled))))))))

(event Custom|Defeated
  (Rendering|Components|Sprite|SetSprite (Variables|Default|GetPaperSprite) (Variables|Default|GetDefeatedSprite))
  (CallFunction|SetCrossVisibility false))

(event EventBeginPlay
  (CallFunction|SetCrossVisibility false)
  (Variables|Default|SetAs%20GM%20Duel (.AsGM%20Duel (Utilities|Casting|CastToGM_Duel (Game|GetGameMode))))
  (Variables|Default|SetSlideEndPos (Variables|/Script/Engine.SceneComponent|GetRelativeLocation (Variables|Default|GetPaperSprite)))
  (CallFunction|Slidein))

(fn ConstructionScript)

(fn SetCrossVisibility
  (params (bNewVisibility :type Boolean))
  (Rendering|SetVisibility (Variables|Default|GetCross) bNewVisibility false))

(fn ResetGame
  (Rendering|Components|Sprite|SetSprite (Variables|Default|GetPaperSprite) (Variables|Default|GetIdleSprite))
  (Variables|Default|SetPressedDraw false)
  (CallFunction|Slidein)
  (CallFunction|SetCrossVisibility false))