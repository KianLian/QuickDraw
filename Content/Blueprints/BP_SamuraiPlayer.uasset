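; BP_SamuraiPlayer is the player-controlled samurai, set up for duel input and viewed through a camera actor in the level.
; On BeginPlay it possesses itself with player controller 0, adds the IMC_Duel Enhanced Input mapping context and switches the view to the first CameraActor found.
; The IA_Attack input prints a debug string and calls Attack, which is defined outside these graphs.
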(event Input|EnhancedActionEvents|EnhancedInputActionIA_Attack
  (params (ActionValue :type Boolean) (ElapsedSeconds :type Float%20%28double-precision%29) (TriggeredSeconds :type Float%20%28double-precision%29) (InputAction :type Input%20Action%20Object%20Reference :default "/Game/Blueprints/Inputs/IA_Attack.IA_Attack"))
  (Development|PrintString "Attack")
  (CallFunction|Attack))

(event EventBeginPlay
  (|CallParentFunction)
  (Pawn|Possess (Game|GetPlayerController 0) self)
  (bind _asplayer_controller (Utilities|Casting|CastToPlayerController (Pawn|GetController)))
  (Input|AddMappingContext (PlayerController|LocalPlayerSubsystems|GetEnhancedInputLocalPlayerSubsystem _asplayer_controller) "/Game/Blueprints/Inputs/IMC_Duel.IMC_Duel" 0 "(bIgnoreAllPressedKeysUntilRelease=True,bForceImmediately=False,bNotifyUserSettings=False)")
  (bind _returnvalue (Actor|GetActorOfClass "/Script/Engine.CameraActor"))
  (Game|Player|SetViewTargetwithBlend (Game|GetPlayerController 0) _returnvalue 0.0 "VTBlend_Linear" 0.0 false))

(fn ConstructionScript
  (|CallParentFunction))