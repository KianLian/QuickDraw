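; Game mode for a samurai quick-draw duel between player and NPC, opening with intro music and a UI menu.
; StartGame finds the duel actors and runs a looping timer that moves Intro to Wait, then after a random delay to Draw.
; Draw fires CallDrawPhaseStarted and shows the exclamation mark.
; Helper functions finish the round, defeat the loser and hide the mark, or reset phase, time and both fighters.
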(event Custom|StartGame
  (bind _returnvalue (Actor|GetActorOfClass "/Game/Blueprints/Bp_ExclamationMark.Bp_ExclamationMark_C"))
  (Variables|Default|SetMark _returnvalue)
  (bind _returnvalue_2 (Actor|GetActorOfClass "/Game/Blueprints/BP_SamuraiPlayer.BP_SamuraiPlayer_C"))
  (Variables|Anims|SetPlayer _returnvalue_2)
  (bind _returnvalue_3 (Actor|GetActorOfClass "/Game/Blueprints/BP_Samurai_NPC.BP_Samurai_NPC_C"))
  (Variables|Anims|SetNPC _returnvalue_3)
  (Utilities|Time|SetTimerbyEvent (delegate Custom|Game%20running) 0.01 true))

(event Custom|Game%20running
  (bind _output_get (Variables|Default|SetElapsedTime (+ 0.01 (Variables|Default|GetElapsedTime))))
  (switch Utilities|FlowControl|Switch|SwitchonE_Phase (Variables|Default|GetPhase)
    (:NewEnumerator0
      (if (>= _output_get (Variables|Default|GetRoundStartTime))
        (Variables|Default|SetPhase "NewEnumerator1")
        (Utilities|FlowControl|Delay (Math|Random|RandomFloatinRange (Variables|Default|GetMinDrawDelay) (Variables|Default|GetMaxDrawDelay)))
        (Variables|Default|SetPhase "NewEnumerator2")
        (Default|CallDrawPhaseStarted)
        (Utilities|IsValid (Variables|Default|GetMark)
          (:Is%20Valid
            _)
          (:Is%20Not%20Valid
            (bind _returnvalue (Game|SpawnActorfromClass "/Game/Blueprints/Bp_ExclamationMark.Bp_ExclamationMark_C" (Variables|Default|GetSpawn%20Transform) "Undefined" "MultiplyWithRoot" 0 0))
            (Variables|Default|SetMark _returnvalue)))
        (Default|SetVisibility (Variables|Default|GetMark) true)))))

(event EventBeginPlay
  (bind _returnvalue (Game|GetPlayerController 0))
  (Audio|PlaySound2D "/Game/Assets/Music/stomps-intro-rhythm-hammer-258072.stomps-intro-rhythm-hammer-258072" 1.0 1.0 0.0 0 0)
  (bind _returnvalue_2 (UserInterface|CreateWidget "/Game/UIMenu.UIMenu_C"))
  (Widget|SetVisibility _returnvalue_2 "Visible")
  (UserInterface|Viewport|AddtoViewport _returnvalue_2 0)
  (Variables|/Script/Engine.PlayerController|SetbShowMouseCursor _returnvalue true)
  (Input|SetInputModeUIOnly _returnvalue 0 "DoNotLock" false))

(event EventTick
  (params (DeltaSeconds :type Float%20%28single-precision%29)))

(fn ConstructionScript)

(fn SetGameFinish
  (Variables|Default|SetPhase "NewEnumerator3"))

(fn AttackSuccesfully
  (params (IsPlayer :type Boolean))
  (if IsPlayer
    (Default|Defeated (Variables|Anims|GetNPC))
    (else
      (Default|Defeated (Variables|Anims|GetPlayer))))
  (Utilities|IsValid (Variables|Default|GetMark)
    (:Is%20Valid
      (Default|SetVisibility (Variables|Default|GetMark) false)
      (Utilities|Time|SetTimerbyEvent (EventDispatchers|CreateEvent :!event Reset) 3.0))))

(fn Reset
  (Variables|Default|SetPhase "NewEnumerator0")
  (Variables|Default|SetElapsedTime 0.0)
  (Default|ResetGame (Variables|Anims|GetPlayer))
  (Default|ResetGame (Variables|Anims|GetNPC)))